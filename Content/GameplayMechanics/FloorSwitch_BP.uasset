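; Floor switch actor that raises and lowers a door in response to RaiseDoor and LowerDoor events, whose trigger is not in this graph.
; RaiseDoor plays the DoorOpenClose timeline, whose DoorElevation track offsets the door's Z from DoorInitialPosition, and LowerDoor reverses it.
; An older MoveComponentTo approach that also moved the switch plate is left disconnected, so only the door moves here.
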(event `self.RaiseDoor`
  (bind (_direction _door_elevation) (`Timeline|Door Open Close` :`NewTime` (`GameplayStatics.GetWorldDeltaSeconds`) :!label _label)
    (:`Update`
      (`SceneComponent.K2_SetRelativeLocation` (`self.Door`) (+ (`KismetMathLibrary.MakeVector` 0.0 0.0 _door_elevation) (`self.DoorInitialPosition`)) false false))))

(event `self.LowerDoor`
  (goto _label :!via `Reverse`))

(fn `UserConstructionScript`)